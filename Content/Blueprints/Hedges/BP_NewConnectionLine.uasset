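; BP_NewConnectionLine is an actor that displays one or two electric beam effects as a connection line.
; On BeginPlay it moves its End component to a configured relative location, feeds that world position to ElectricLine's BeamEnd parameter and activates it.
; If SecondBeam is set, ElectricLine1 also activates, with its end computed from the actor's forward vector, an angle and a length.
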(event `self.ReceiveBeginPlay`
  (bind _electricline (`self.ElectricLine`))
  (bind _end (`self.End`))
  (bind _electricline1 (`self.ElectricLine1`))
  (`SceneComponent.K2_SetRelativeLocation` _end (`self.FirstBeamEndLocation`) false false)
  (`FXSystemComponent.SetVectorParameter` _electricline "BeamEnd" (`SceneComponent.K2_GetComponentLocation` _end))
  (`ActorComponent.Activate` _electricline false)
  (if (`self.bSecondBeam`)
    (`FXSystemComponent.SetVectorParameter` _electricline1 "BeamEnd" (+ (* (`KismetMathLibrary.GreaterGreater_VectorRotator` (`self.GetActorForwardVector`) (`self.SecondBeamAngle`)) (`self.SecondBeamLength`)) (`self.K2_GetActorLocation`)))
    (`ActorComponent.Activate` _electricline1 false)))

(fn `UserConstructionScript`)