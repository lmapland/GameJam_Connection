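; BP_Melee_Blue is a melee warrior enemy variant that adds electric arc effects, apparently for its death.
; StartElectricParticles attaches Niagara arcs to head, shoulder, elbow and back sockets, setting each beam end once to the Sock_Beneath location at spawn.
; The spawned systems are kept in NSElectrics, which EndElectricParticles destroys and clears.
; Neither event is called in this graph, and the construction script only calls the parent.
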(event `self.StartElectricParticles`
  (`|ExecutionSequence`
    (:`then_0`
      (bind _returnvalue (`NiagaraFunctionLibrary.SpawnSystemAttached` "/Game/Assets/ParticleEffects/OrcDeath/NS_ElectricArcsDeath.NS_ElectricArcsDeath" (`self.Mesh`) "Sock_Head" (0.0 0.0 0.0) (struct) "KeepRelativeOffset"))
      (`FXSystemComponent.SetVectorParameter` _returnvalue "BeamEnd" (`SceneComponent.GetSocketLocation` (`self.Mesh`) "Sock_Beneath"))
      (`KismetArrayLibrary.Array_Add` (`self.NSElectrics`) _returnvalue))
    (:`then_1`
      (bind _returnvalue_2 (`NiagaraFunctionLibrary.SpawnSystemAttached` "/Game/Assets/ParticleEffects/OrcDeath/NS_ElectricArcsDeath.NS_ElectricArcsDeath" (`self.Mesh`) "Sock_ShoulderR" (0.0 0.0 0.0) (struct) "KeepRelativeOffset"))
      (`FXSystemComponent.SetVectorParameter` _returnvalue_2 "BeamEnd" (`SceneComponent.GetSocketLocation` (`self.Mesh`) "Sock_Beneath"))
      (`KismetArrayLibrary.Array_Add` (`self.NSElectrics`) _returnvalue_2))
    (:`then_2`
      (bind _returnvalue_3 (`NiagaraFunctionLibrary.SpawnSystemAttached` "/Game/Assets/ParticleEffects/OrcDeath/NS_ElectricArcsDeath.NS_ElectricArcsDeath" (`self.Mesh`) "Sock_ElbowL" (0.0 0.0 0.0) (struct) "KeepRelativeOffset"))
      (`FXSystemComponent.SetVectorParameter` _returnvalue_3 "BeamEnd" (`SceneComponent.GetSocketLocation` (`self.Mesh`) "Sock_Beneath"))
      (`KismetArrayLibrary.Array_Add` (`self.NSElectrics`) _returnvalue_3))
    (:`then_3`
      (bind _returnvalue_4 (`NiagaraFunctionLibrary.SpawnSystemAttached` "/Game/Assets/ParticleEffects/OrcDeath/NS_ElectricArcsDeath.NS_ElectricArcsDeath" (`self.Mesh`) "Sock_Back" (0.0 0.0 0.0) (struct) "KeepRelativeOffset"))
      (`FXSystemComponent.SetVectorParameter` _returnvalue_4 "BeamEnd" (`SceneComponent.GetSocketLocation` (`self.Mesh`) "Sock_Beneath"))
      (`KismetArrayLibrary.Array_Add` (`self.NSElectrics`) _returnvalue_4))))

(event `self.EndElectricParticles`
  (for _array_element (`self.NSElectrics`)
    (`ActorComponent.K2_DestroyComponent` _array_element))
  (`KismetArrayLibrary.Array_Clear` (`self.NSElectrics`)))

(fn `UserConstructionScript`
  (`parent.UserConstructionScript`))