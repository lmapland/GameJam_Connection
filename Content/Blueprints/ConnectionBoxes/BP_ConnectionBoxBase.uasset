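; BP_ConnectionBoxBase is a base actor for a pair of boxes that visually join when connected.
; ConnectBoxes deactivates its Niagara effect and plays a timeline that slides UnconnectedBox along its relative X axis.
; When the timeline finishes, it applies a base color material to both boxes if IsReady, then calls BoxesAreConnected.
; BeginPlay draws a temporary debug sphere slightly above the actor.
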(event `self.ReceiveBeginPlay`
  (`KismetSystemLibrary.DrawDebugSphere` (+ (`self.K2_GetActorLocation`) (0.0 0.0 60.0)) 5.0 8 (struct :`G` 0.069328 :`B` 1.0 :`A` 1.0) 30.0 1.0))

(event `self.ConnectBoxes`
  (bind _unconnectedbox (`self.UnconnectedBox`))
  (`ActorComponent.Deactivate` (`self.Niagara`))
  (bind (_direction _boxmovementx) (`Timeline|BoxConnectTimeline`)
    (:`Update`
      (`SceneComponent.K2_SetRelativeLocation` _unconnectedbox (`KismetMathLibrary.MakeVector` _boxmovementx (.y (`SceneComponent.RelativeLocation` _unconnectedbox)) (.z (`SceneComponent.RelativeLocation` _unconnectedbox))) false false))
    (:`Finished`
      (if (`self.bIsReady`)
        (`self.FillWithColor`))
      (`self.BoxesAreConnected`))))

(event `self.FillWithColor`
  (`PrimitiveComponent.SetMaterial` (`self.ConnectedBox`) 0 "/Game/Swamp_Forest/materials/plants_materials/M_base_color.M_base_color")
  (`PrimitiveComponent.SetMaterial` (`self.UnconnectedBox`) 0 "/Game/Swamp_Forest/materials/plants_materials/M_base_color.M_base_color"))

(fn `UserConstructionScript`)